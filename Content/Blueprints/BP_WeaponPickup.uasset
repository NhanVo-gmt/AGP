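; BP_WeaponPickup is a weapon pickup whose mesh material reflects the weapon's rarity.
; The UpdateWeaponPickupMaterial event checks WeaponRarity through nested branches and sets PickupMesh slot 0 to the Common, Rare, Master or Legendary material, with Legendary as the fallback.
; BeginPlay, overlap, Tick and the construction script do nothing, and nothing in this Blueprint calls the update event.
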(event `self.UpdateWeaponPickupMaterial`
  (if (`|EnumEquality` (`self.WeaponRarity`) "Common")
    (`PrimitiveComponent.SetMaterial` (`self.PickupMesh`) 0 "/Game/Materials/CommonMaterial.CommonMaterial")
    (elif (`|EnumEquality` (`self.WeaponRarity`) "Rare")
      (`PrimitiveComponent.SetMaterial` (`self.PickupMesh`) 0 "/Game/Materials/RareMaterial.RareMaterial")
      (elif (`|EnumEquality` (`self.WeaponRarity`) "Master")
        (`PrimitiveComponent.SetMaterial` (`self.PickupMesh`) 0 "/Game/Materials/MasterMaterial.MasterMaterial")
        (else
          (`PrimitiveComponent.SetMaterial` (`self.PickupMesh`) 0 "/Game/Materials/LegendaryMaterial.LegendaryMaterial"))))))

(fn `UserConstructionScript`)